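; Timed grenade actor that explodes two seconds after BeginPlay with a particle effect and sound, then hides its Sphere component.
; A Damage event runs a multi sphere trace for Pawns around the Sphere, with debug drawing left on.
; Hit actors are deduplicated with AddUnique, so each takes flat damage once, without distance falloff.
; The actor lingers briefly after the blast, then destroys itself.
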(event Custom|Damage
  (bind _sphere (Variables|Default|GetSphere))
  (bind _returnvalue (Transformation|GetWorldLocation _sphere))
  (bind (_outhits _returnvalue_2) (Collision|MultiSphereTraceForObjects _returnvalue _returnvalue 3.5e+02 (Utilities|Array|MakeArray "ObjectTypeQuery3") false 0 "ForDuration"))
  (if _returnvalue_2
    (for _array_element _outhits
      (Utilities|Array|AddUnique (Variables|Default|GetHitActors) (.HitActor (Collision|BreakHitResult _array_element))))
    (for _array_element_2 (Variables|Default|GetHitActors)
      (Game|Damage|ApplyDamage _array_element_2 1e+02 0 self))))

(event EventBeginPlay
  (Utilities|FlowControl|Delay 2.0)
  (Effects|SpawnEmitteratLocation "/Game/StarterContent/Particles/P_Explosion.P_Explosion" (Transformation|GetActorLocation) "0, 0, 0" "2.000000,2.000000,2.000000")
  (Audio|PlaySoundatLocation "/Game/StarterContent/Audio/Explosion_Cue.Explosion_Cue" (Transformation|GetActorLocation) "0, 0, 0" 2.0 1.0 0.0 "/Game/Audio/Enemy/SA_HIt.SA_HIt" 0 0 0)
  (Development|SetHiddeninGame (Variables|Default|GetSphere) true false)
  (CallFunction|Damage)
  (Utilities|FlowControl|Delay 3.0)
  (Actor|DestroyActor))

(fn ConstructionScript)