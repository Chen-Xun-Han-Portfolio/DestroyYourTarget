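; BP_ProtectObject is a destructible objective the player must protect, whose destruction triggers game over.
; Damage received before game over lowers its clamped health and updates a WB_HealthBar widget.
; At zero health it swaps its static mesh for a Geometry Collection and spawns an exploding BP_Bomb there.
; It also flags one melee enemy dead, calls the player's GameOver, then destroys itself after a short delay.
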(event EventBeginPlay
  (CallFunction|UpdateHealthBar))

(event Game|Damage|EventAnyDamage
  (params (Damage :type Float%20%28single-precision%29) (DamageType :type Damage%20Type%20Object%20Reference) (InstigatedBy :type Controller%20Object%20Reference) (DamageCauser :type Actor%20Object%20Reference))
  (bind _asbp_player (Utilities|Casting|CastToBP_Player (Game|GetPlayerCharacter 0)))
  (if (not (Variables|/Game/Blueprint/BP_Player.BP_Player_C|GetGameOver? _asbp_player))
    (bind _output_get (Variables|Default|SetHealth (Math|Float|Clamp(Float) (- (Variables|Default|GetHealth) Damage) 0.0 1e+02)))
    (Development|PrintString (Utilities|String|ToString(Float) _output_get))
    (CallFunction|UpdateHealthBar)
    (if (== (Variables|Default|GetHealth) 0.0)
      (Utilities|FlowControl|DoOnce false
        (:Completed
          (Components|DestroyComponent (Variables|Default|GetStaticMesh))
          (bind _returnvalue (AddComponent|AddGeometryCollectionComponent false))
          (bind _returnvalue_2 (Game|SpawnActorfromClass "/Game/Blueprint/BP_Bomb.BP_Bomb_C" (Math|Transform|MakeTransform (Transformation|GetWorldLocation _returnvalue) (Transformation|GetWorldRotation _returnvalue) "1.000000,1.000000,1.000000") "Undefined" "MultiplyWithRoot" 0 0))
          (Default|Explode _returnvalue_2)
          (bind _returnvalue_3 (Actor|GetActorOfClass "/Game/Blueprint/Enemies/BP_Enemy_Melee.BP_Enemy_Melee_C"))
          (Variables|/Game/Blueprint/Enemies/BP_Enemy_Melee.BP_Enemy_Melee_C|SetisDead? _returnvalue_3 true)
          (bind _returnvalue_4 (Actor|GetActorOfClass "/Game/Blueprint/BP_Player.BP_Player_C"))
          (Default|GameOver _returnvalue_4)
          (Utilities|FlowControl|Delay 3.0)
          (Actor|DestroyActor))))))

(fn ConstructionScript)

(fn UpdateHealthBar
  (bind _aswb_health_bar (Utilities|Casting|CastToWB_HealthBar (UserInterface|GetUserWidgetObject (Variables|Default|GetHealthBar))))
  (Utilities|IsValid _aswb_health_bar
    (:Is%20Valid
      (Variables|/Game/WidgetBP/WB_HealthBar.WB_HealthBar_C|SetHealth _aswb_health_bar (Variables|Default|GetHealth))
      (return))))