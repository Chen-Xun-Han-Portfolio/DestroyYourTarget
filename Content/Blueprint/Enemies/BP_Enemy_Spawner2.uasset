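; BP_Enemy_Spawner2 is a one-shot spawner actor that introduces a melee enemy with a spawn effect.
; On BeginPlay it plays a Niagara effect, waits briefly, spawns BP_Enemy_Melee at its Billboard's location, then destroys itself.
; EnemyIncreaseByTime sets a Delay variable from the player's Minutes and Seconds, but the event graph neither calls it nor uses that variable.
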(event EventBeginPlay
  ;[1 1 1] Start Spawn
  (Niagara|SpawnSystematLocation "/Game/FX/NS_Spawn.NS_Spawn" (.location (Transformation|GetActorTransform)))
  (Utilities|FlowControl|Delay 1.0)
  (Game|SpawnActorfromClass "/Game/Blueprint/Enemies/BP_Enemy_Melee.BP_Enemy_Melee_C" (Math|Transform|MakeTransform (Transformation|GetWorldLocation (Variables|Default|GetBillboard)) "0, 0, 0" "1.000000,1.000000,1.000000") "AdjustIfPossibleButAlwaysSpawn" "MultiplyWithRoot" 0 0)
  (Development|PrintString "Spawn")
  (Actor|DestroyActor))

(fn ConstructionScript)

(fn EnemyIncreasebyTime
  (bind _asbp_player (Utilities|Casting|CastToBP_Player (Game|GetPlayerCharacter 0)))
  (if (and (== (Variables|/Game/Blueprint/BP_Player.BP_Player_C|GetMinutes _asbp_player) 1) (<= (Variables|/Game/Blueprint/BP_Player.BP_Player_C|GetSeconds _asbp_player) 59))
    (bind _output_get (Variables|Default|Setdelay 4))
    (Development|PrintString (Utilities|String|ToString(Integer) _output_get))
    (elif (and (== (Variables|/Game/Blueprint/BP_Player.BP_Player_C|GetMinutes _asbp_player) 0) (<= (Variables|/Game/Blueprint/BP_Player.BP_Player_C|GetSeconds _asbp_player) 59))
      (bind _output_get_2 (Variables|Default|Setdelay 3))
      (Development|PrintString (Utilities|String|ToString(Integer) _output_get_2))
      (else
        (bind _output_get_3 (Variables|Default|Setdelay 2))
        (Development|PrintString (Utilities|String|ToString(Integer) _output_get_3)))))
  (return))