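; Melee enemy that hunts the BP_ProtectObject and slashes it until killed.
; A ChaseTarget loop uses AI MoveTo, then plays a slash montage whose notify runs a forward sphere trace to apply damage and a hit sound, repeating after a delay.
; Incoming damage, ignored once the player's game is over, lowers health and updates a widget health bar.
; At zero it ragdolls, increments the player's score and destroys itself.
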(event Custom|Die
  (bind _mesh (Variables|Character|GetMesh))
  ;[1 1 1] Die
  (Variables|Default|SetisDead? true)
  (Physics|SetSimulatePhysics _mesh true)
  (Collision|SetCollisionEnabled _mesh "QueryAndPhysics")
  (Collision|SetCollisionEnabled (Variables|Collision|GetCapsuleComponent) "NoCollision")
  (bind _asbp_player (Utilities|Casting|CastToBP_Player (Game|GetPlayerCharacter 0)))
  (Math|Integer|IncrementInt (Variables|/Game/Blueprint/BP_Player.BP_Player_C|GetScore _asbp_player)
    (:%20%20
      (Utilities|FlowControl|Delay 2.0)
      ;;[1 1 1] Need put at end
      (Actor|DestroyActor))))

(event Custom|ChaseTarget
  ;[1 1 1] Attack Player
  (if (Variables|Default|GetisDead?)
    (Development|PrintString "Dead")
    (else
      (bind _returnvalue (Actor|GetActorOfClass "/Game/Blueprint/BP_ProtectObject.BP_ProtectObject_C"))
      (AI|AIMoveTo self "0, 0, 0" _returnvalue 3e+02 false
        (:OnSuccess
          (CallFunction|Attack)
          (Utilities|FlowControl|Delay 2.0))
        (:OnFail
          _))
      (CallFunction|ChaseTarget))))

(event Custom|Attack
  (bind _returnvalue (Transformation|GetActorLocation))
  ;[1 1 1] Attack Player
  (if (Variables|Default|GetisDead?)
    (Development|PrintString "NoAttack")
    (else
      (bind _returnvalue_2 (Actor|GetActorOfClass "/Game/Blueprint/BP_ProtectObject.BP_ProtectObject_C"))
      (Utilities|IsValid _returnvalue_2
        (:Is%20Valid
          (Transformation|SetActorRotation (Math|Rotator|MakeRotator 0.0 0.0 (.yaw (Math|Rotator|FindLookatRotation (Transformation|GetActorLocation) (Transformation|GetActorLocation _returnvalue_2)))))
          (bind _notifyname (Animation|Montage|PlayMontage (Variables|Character|GetMesh) "/Game/Animation/Enemy/Enemy_Slash_Montage.Enemy_Slash_Montage")
            (:OnNotifyBegin
              (switch name _notifyname
                (:Slash
                  (bind (_outhit _returnvalue_3) (Collision|SphereTraceForObjects _returnvalue (+ _returnvalue (* (Transformation|GetActorForwardVector) 2e+02)) 2e+01 (Utilities|Array|MakeArray "ObjectTypeQuery2") false 0 "ForDuration"))
                  (if _returnvalue_3
                    (bind _asbp_protect_object (Utilities|Casting|CastToBP_ProtectObject (.HitActor (Collision|BreakHitResult _outhit))))
                    (Game|Damage|ApplyDamage _asbp_protect_object 1e+01 0 self)
                    (Audio|PlaySoundatLocation "/Game/Audio/Enemy/582371__quatricise__axe-hits-2.582371__quatricise__axe-hits-2" (Transformation|GetActorLocation) "0, 0, 0" 1.0 1.0 0.0 "/Game/Audio/Enemy/SA_HIt.SA_HIt" 0 0 0)))))))))))

(event EventBeginPlay
  (CallFunction|UpdateHealthBar)
  (CallFunction|ChaseTarget))

(event Game|Damage|EventAnyDamage
  (params (Damage :type Float%20%28single-precision%29) (DamageType :type Damage%20Type%20Object%20Reference) (InstigatedBy :type Controller%20Object%20Reference) (DamageCauser :type Actor%20Object%20Reference))
  ;[1 1 1] Recieve Damage
  (bind _returnvalue (Actor|GetActorOfClass "/Game/Blueprint/BP_Player.BP_Player_C"))
  (if (not (Variables|/Game/Blueprint/BP_Player.BP_Player_C|GetGameOver? _returnvalue))
    (bind _output_get (Variables|Default|SetHealth (Math|Float|Clamp(Float) (- (Variables|Default|GetHealth) Damage) 0.0 1e+02)))
    (Development|PrintString (Utilities|String|ToString(Float) _output_get))
    (CallFunction|UpdateHealthBar)
    (if (== (Variables|Default|GetHealth) 0.0)
      (CallFunction|Die))))

(fn ConstructionScript)

(fn UpdateHealthBar
  (bind _aswb_health_bar (Utilities|Casting|CastToWB_HealthBar (UserInterface|GetUserWidgetObject (Variables|Default|GetHealthBar))))
  (Utilities|IsValid _aswb_health_bar
    (:Is%20Valid
      (Variables|/Game/WidgetBP/WB_HealthBar.WB_HealthBar_C|SetHealth _aswb_health_bar (Variables|Default|GetHealth))
      (return))))