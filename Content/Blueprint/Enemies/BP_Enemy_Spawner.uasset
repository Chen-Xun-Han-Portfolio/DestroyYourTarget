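; Enemy spawner actor that, when spawning is allowed, spawns a melee enemy at its billboard after a delayed Niagara effect on BeginPlay.
; It then binds to the game mode's respawn-enemy event, which replays the delayed effect and spawns a batch of enemies.
; After each batch, it reads the player's timer to update the next batch size, giving more enemies at zero minutes than at one.
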(event Custom|SpawnEnemy
  (Utilities|FlowControl|Delay 1.0)
  (Niagara|SpawnSystematLocation "/Game/FX/NS_Spawn.NS_Spawn" (.location (Transformation|GetActorTransform)))
  (Utilities|FlowControl|Delay 1.0)
  (for _index (range 0 (- (Variables|Default|GetEnemySpawned) 1))
    (Game|SpawnActorfromClass "/Game/Blueprint/Enemies/BP_Enemy_Melee.BP_Enemy_Melee_C" (Math|Transform|MakeTransform (Transformation|GetWorldLocation (Variables|Default|GetBillboard)) "0, 0, 0" "1.000000,1.000000,1.000000") "AdjustIfPossibleButAlwaysSpawn" "MultiplyWithRoot" 0 0))
  (CallFunction|EnemyIncreasebyTime))

(event EventBeginPlay
  (if (Variables|Default|GetAllowSpawn)
    (bind _asbp_third_person_game_mode (Utilities|Casting|CastToBP_ThirdPersonGameMode (Game|GetGameMode)))
    (Utilities|FlowControl|Delay 1.0)
    (Niagara|SpawnSystematLocation "/Game/FX/NS_Spawn.NS_Spawn" (.location (Transformation|GetActorTransform)))
    (Utilities|FlowControl|Delay 1.0)
    (Game|SpawnActorfromClass "/Game/Blueprint/Enemies/BP_Enemy_Melee.BP_Enemy_Melee_C" (Math|Transform|MakeTransform (Transformation|GetWorldLocation (Variables|Default|GetBillboard)) "0, 0, 0" "1.000000,1.000000,1.000000") "AdjustIfPossibleButAlwaysSpawn" "MultiplyWithRoot" 0 0)
    (Development|PrintString "Spawn")
    (EventDispatchers|BindEventtoRespawnEnemy _asbp_third_person_game_mode (delegate Custom|SpawnEnemy))))

(fn ConstructionScript)

(fn EnemyIncreasebyTime
  (bind _asbp_player (Utilities|Casting|CastToBP_Player (Game|GetPlayerCharacter 0)))
  (if (and (== (Variables|/Game/Blueprint/BP_Player.BP_Player_C|GetMinutes _asbp_player) 1) (<= (Variables|/Game/Blueprint/BP_Player.BP_Player_C|GetSeconds _asbp_player) 59))
    (Variables|Default|SetEnemySpawned 2)
    (Development|PrintString "+2")
    (return)
    (elif (and (== (Variables|/Game/Blueprint/BP_Player.BP_Player_C|GetMinutes _asbp_player) 0) (<= (Variables|/Game/Blueprint/BP_Player.BP_Player_C|GetSeconds _asbp_player) 59))
      (Variables|Default|SetEnemySpawned 3)
      (return))))